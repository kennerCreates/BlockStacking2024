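; Player pawn for a free-floating camera that moves along the camera's forward and right vectors using Enhanced Input.
; On possession by the player controller it adds the floating-camera mapping context for move, look and block spawning.
; Spawn input messages every registered World to spawn a physics block.
; A looping timer checks position and teleports the pawn to the opposite side when it leaves the WorldSize bounds on any axis.
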(event Custom|CheckPlayerAtEdge
  (bind _output_get (Variables|Default|SetPlayerTransform (Transformation|GetActorTransform)))
  (Variables|Default|SetPlayerX (.x (.location _output_get)))
  (Variables|Default|SetPlayerY (.y (.location _output_get)))
  (Variables|Default|SetPlayer%20Z (.z (.location _output_get)))
  (CallFunction|TeleportPlayerOutsideBounds))

(event Input|EnhancedActionEvents|EnhancedInputActionIA_Look
  (params (ActionValue :type Vector%202D%20Structure) (ElapsedSeconds :type Float%20%28double-precision%29) (TriggeredSeconds :type Float%20%28double-precision%29) (InputAction :type Input%20Action%20Object%20Reference :default "/Game/GamePlay/Input/Actions/IA_Look.IA_Look"))
  (Pawn|Input|AddControllerYawInput (.x ActionValue))
  (Pawn|Input|AddControllerPitchInput (* (.y ActionValue) -1.0)))

(event Input|EnhancedActionEvents|EnhancedInputActionIA_Move
  (params (ActionValue :type Vector%202D%20Structure) (ElapsedSeconds :type Float%20%28double-precision%29) (TriggeredSeconds :type Float%20%28double-precision%29) (InputAction :type Input%20Action%20Object%20Reference :default "/Game/GamePlay/Input/Actions/IA_Move.IA_Move"))
  (bind _camera (Variables|Default|GetCamera))
  (Pawn|Input|AddMovementInput (Math|Vector|GetForwardVector _camera) (.y ActionValue) false)
  (Pawn|Input|AddMovementInput (Math|Vector|GetRightVector _camera) (.x ActionValue) false))

(event Input|EnhancedActionEvents|EnhancedInputActionIA_SpawnBlock
  (params (ActionValue :type Boolean) (ElapsedSeconds :type Float%20%28double-precision%29) (TriggeredSeconds :type Float%20%28double-precision%29) (InputAction :type Input%20Action%20Object%20Reference :default "/Game/GamePlay/Input/Actions/IA_SpawnBlock.IA_SpawnBlock"))
  (:Started
    (for _array_element (Variables|Default|GetWorlds)
      (Class|BPIWorlds|SpawnPhysicsBlock(Message) _array_element))))

(event EventControllerChanged
  (params (OldController :type Controller%20Object%20Reference) (NewController :type Controller%20Object%20Reference))
  (bind _asbp_controller_player (Utilities|Casting|CastToBP_Controller_Player NewController))
  (Input|AddMappingContext (PlayerController|LocalPlayerSubsystems|GetEnhancedInputLocalPlayerSubsystem _asbp_controller_player) "/Game/GamePlay/Input/IMC_FloatingCamera.IMC_FloatingCamera" 0 "(bIgnoreAllPressedKeysUntilRelease=True,bForceImmediately=False,bNotifyUserSettings=False)"))

(event EventBeginPlay
  (Utilities|Time|SetTimerbyEvent (delegate Custom|CheckPlayerAtEdge) 0.25 true))

(event EventSendWorldtoPlayer
  (params (World :type BP%20Interactable%20World%20Object%20Reference))
  (Utilities|Array|Add (Variables|Default|GetWorlds) World))

(fn ConstructionScript)

(fn TeleportPlayerOutsideBounds
  (bind _playertransform (Variables|Default|GetPlayerTransform))
  (bind _playertransform_2 (Variables|Default|GetPlayerTransform))
  (bind _playertransform_3 (Variables|Default|GetPlayerTransform))
  (bind _playertransform_4 (Variables|Default|GetPlayerTransform))
  (bind _playertransform_5 (Variables|Default|GetPlayerTransform))
  (bind _playertransform_6 (Variables|Default|GetPlayerTransform))
  (if (>= (Variables|Default|GetPlayerX) (Variables|Default|GetWorldSize))
    (Transformation|SetActorTransform (Math|Transform|MakeTransform (Math|Vector|MakeVector (* (Variables|Default|GetWorldSize) -1.0) (.y (.location _playertransform_2)) (.z (.location _playertransform_2))) (.rotation _playertransform_2) (.scale _playertransform_2)))
    (elif (<= (Variables|Default|GetPlayerX) (* (Variables|Default|GetWorldSize) -1.0))
      (Transformation|SetActorTransform (Math|Transform|MakeTransform (Math|Vector|MakeVector (Variables|Default|GetWorldSize) (.y (.location _playertransform_3)) (.z (.location _playertransform_3))) (.rotation _playertransform_3) (.scale _playertransform_3)))))
  (if (>= (Variables|Default|GetPlayerY) (Variables|Default|GetWorldSize))
    (Transformation|SetActorTransform (Math|Transform|MakeTransform (Math|Vector|MakeVector (.x (.location _playertransform_4)) (* (Variables|Default|GetWorldSize) -1.0) (.z (.location _playertransform_4))) (.rotation _playertransform_4) (.scale _playertransform_4)))
    (elif (<= (Variables|Default|GetPlayerY) (* (Variables|Default|GetWorldSize) -1.0))
      (Transformation|SetActorTransform (Math|Transform|MakeTransform (Math|Vector|MakeVector (.x (.location _playertransform_5)) (Variables|Default|GetWorldSize) (.z (.location _playertransform_5))) (.rotation _playertransform_5) (.scale _playertransform_5)))))
  (if (>= (Variables|Default|GetPlayer%20Z) (Variables|Default|GetWorldSize))
    (Transformation|SetActorTransform (Math|Transform|MakeTransform (Math|Vector|MakeVector (.x (.location _playertransform_6)) (.y (.location _playertransform_6)) (* (Variables|Default|GetWorldSize) -1.0)) (.rotation _playertransform_6) (.scale _playertransform_6)))
    (elif (<= (Variables|Default|GetPlayer%20Z) (* (Variables|Default|GetWorldSize) -1.0))
      (Transformation|SetActorTransform (Math|Transform|MakeTransform (Math|Vector|MakeVector (.x (.location _playertransform)) (.y (.location _playertransform)) (Variables|Default|GetWorldSize)) (.rotation _playertransform) (.scale _playertransform))))))