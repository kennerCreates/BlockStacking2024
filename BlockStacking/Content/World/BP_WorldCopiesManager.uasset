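; World manager that surrounds the level's BP_InteractableWorld with a square grid of spawned copies, likely to make the world appear to repeat.
; The construction script finds that actor and caches its box half-extent as the tile size.
; BeginPlay lays out (2 × CopiesEachSide + 1)² cells centred on the world origin at Z=0.
; The centre cell spawns nothing and draws a temporary debug sphere instead.
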(event EventBeginPlay
  (bind _worldhalfsize (Variables|Default|GetWorldHalfSize))
  (bind _worldhalfsize_2 (Variables|Default|GetWorldHalfSize))
  (bind _returnvalue (* (.y _worldhalfsize) 2.0))
  (bind _returnvalue_2 (* (.x _worldhalfsize_2) 2.0))
  (Variables|Default|SetTotalCopies (+ (* (Variables|Default|GetCopiesEachSide) 2) 1))
  (for _index (range 0 (- (* (Variables|Default|GetTotalCopies) (Variables|Default|GetTotalCopies)) 1))
    (if (== _index (/ (* (Variables|Default|GetTotalCopies) (Variables|Default|GetTotalCopies)) 2))
      (Rendering|Debug|DrawDebugSphere (Math|Vector|MakeVector (+ (- (* (Math|Integer|%(Integer) _index (Variables|Default|GetTotalCopies)) _returnvalue_2) (/ (* _returnvalue_2 (Variables|Default|GetTotalCopies)) 2.0)) (.x (Variables|Default|GetWorldHalfSize))) (+ (- (* (/ _index (Variables|Default|GetTotalCopies)) _returnvalue) (/ (* _returnvalue (Variables|Default|GetTotalCopies)) 2.0)) (.y (Variables|Default|GetWorldHalfSize))) 0.0) 5e+02 20 "(R=0.049029,G=0.136027,B=1.000000,A=1.000000)" 1.2e+02 1e+01)
      (else
        (Game|SpawnActorfromClass "/Game/World/BP_InteractableWorld.BP_InteractableWorld_C" (Math|Transform|MakeTransform (Math|Vector|MakeVector (+ (- (* (Math|Integer|%(Integer) _index (Variables|Default|GetTotalCopies)) _returnvalue_2) (/ (* _returnvalue_2 (Variables|Default|GetTotalCopies)) 2.0)) (.x (Variables|Default|GetWorldHalfSize))) (+ (- (* (/ _index (Variables|Default|GetTotalCopies)) _returnvalue) (/ (* _returnvalue (Variables|Default|GetTotalCopies)) 2.0)) (.y (Variables|Default|GetWorldHalfSize))) 0.0) "0, 0, 0" "1.000000,1.000000,1.000000") "Undefined" "MultiplyWithRoot" 0 0)))))

(fn ConstructionScript
  (bind _returnvalue (Actor|GetActorOfClass "/Game/World/BP_InteractableWorld.BP_InteractableWorld_C"))
  (bind _output_get (Variables|Default|SetInteractableWorld _returnvalue))
  (Variables|Default|SetWorldHalfSize (Components|Box|GetScaledBoxExtent (Variables|/Game/World/BP_InteractableWorld.BP_InteractableWorld_C|GetBox _output_get))))