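; BP_InteractableWorld is a world actor bounded by a Box component that makes itself known to the player.
; The construction script adds a scaled cube mesh as a floor, offset downward by the box's vertical extent.
; On BeginPlay it draws a long-lived debug outline of the box and passes itself to the first player's pawn through SendWorldToPlayerMessage.
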(event EventBeginPlay
  (bind _box (Variables|Default|GetBox))
  (Rendering|Debug|DrawDebugBox (Transformation|GetWorldLocation _box) (Components|Box|GetScaledBoxExtent _box) "(R=1.000000,G=0.077081,B=0.392109,A=1.000000)" "0, 0, 0" 1.2e+02 5.0)
  (Class|BPIPlayer|SendWorldtoPlayer(Message) (Game|Player|GetPlayerPawn 0) self))

(fn ConstructionScript
  (bind _returnvalue (AddComponent|AddStaticMeshComponent false (Math|Transform|MakeTransform (Math|Vector|MakeVector 0.0 0.0 (* (.Z (Math|Vector|BreakVector (Components|Box|GetScaledBoxExtent (Variables|Default|GetBox)))) -1.0)))))
  (bind _output_get (Variables|Default|SetFloor _returnvalue))
  (Components|StaticMesh|SetStaticMesh _output_get "/Engine/VREditor/BasicMeshes/SM_Cube_02.SM_Cube_02")
  (Transformation|SetWorldScale3D (Variables|Default|GetFloor) "20.000000,20.000000,1.000000"))